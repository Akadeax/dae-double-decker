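; Player controller for the train director, handling drag-and-release placement of train cards with the mouse.
; On begin play it enables cursor input, loads level data by level name from a DataTable and creates the HUD.
; Clicking a card looks up its data and starts a pawn preview that follows the mouse each tick.
; Release decrements that card's level count and has the pawn spawn its effect at the mouse position.
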(event Input|EnhancedActionEvents|EnhancedInputActionIA_Release
  (params (ActionValue :type Boolean) (ElapsedSeconds :type Float%20%28double-precision%29) (TriggeredSeconds :type Float%20%28double-precision%29) (InputAction :type Input%20Action%20Object%20Reference :default "/Game/Player/Input/IA_Release.IA_Release"))
  (if (Variables|Default|GetHoldingTrainCard)
    (CallFunction|DecrementCurrentCard)
    (Default|SpawnCardEffect (Variables|Default|GetTrainControllerPawn) (Variables|Default|GetHeldCard) (Utilities|GetMousePos))
    (Variables|Default|SetHoldingTrainCard false)))

(event EventTick
  (params (DeltaSeconds :type Float%20%28single-precision%29))
  (if (Variables|Default|GetHoldingTrainCard)
    (Default|UpdatePreviewPosition (Variables|Default|GetTrainControllerPawn) (Utilities|GetMousePos))))

(event EventBeginPlay
  (bind _asbp_train_director_pawn (Utilities|Casting|CastToBP_TrainDirectorPawn (Pawn|GetControlledPawn)))
  (Variables|Default|SetTrainControllerPawn _asbp_train_director_pawn)
  (CallFunction|SetupMouseInput)
  (CallFunction|SetupLevelData)
  (CallFunction|SetupHUD))

(fn ConstructionScript)

(fn OnTrainCardClicked
  (params (Card :type Name))
  (bind _carddata (CallFunction|NametoCardData Card))
  (Default|StartPreview (Variables|Default|GetTrainControllerPawn) _carddata)
  (Variables|Default|SetHoldingTrainCard true)
  (Variables|Default|SetHeldCard _carddata))

(fn SetupMouseInput
  (Variables|Default|SetbShowMouseCursor true)
  (Variables|Default|SetbEnableClickEvents true)
  (Variables|Default|SetbEnableMouseOverEvents true)
  (Input|AddMappingContext (PlayerController|LocalPlayerSubsystems|GetEnhancedInputLocalPlayerSubsystem) "/Game/Player/Input/IM_Game.IM_Game" 0 "(bIgnoreAllPressedKeysUntilRelease=True,bForceImmediately=False,bNotifyUserSettings=False)"))

(fn SetupHUD
  (bind _self self)
  (bind _returnvalue (UserInterface|CreateWidget "/Game/Player/WBP_HUD.WBP_HUD_C" _self _self))
  (UserInterface|Viewport|AddtoViewport _returnvalue 0))

(fn NametoCardData
  (params (Name :type Name))
  (bind _returnvalue (Utilities|GetDataTableRow "/Game/Player/Cards/DT_TrainCardData.DT_TrainCardData" Name)
    (:then
      (return _returnvalue))
    (:RowNotFound
      (return ""))))

(fn SetupLevelData
  (bind _returnvalue (Game|GetCurrentLevelName true))
  (bind _returnvalue_2 (Utilities|GetDataTableRow "/Game/Levels/DT_LevelData.DT_LevelData" (Utilities|String|StringToName _returnvalue))
    (:then
      (Variables|Default|SetCurrentLevelData _returnvalue_2))
    (:RowNotFound
      (Development|PrintString "Couldn't find level data"))))

(fn DecrementCurrentCard
  (bind _heldcard (Variables|Default|GetHeldCard))
  (bind _currentleveldata (Variables|Default|GetCurrentLevelData))
  (bind _name (Utilities|Struct|BreakS_TrainCardData _heldcard))
  (bind _cardamounts (Utilities|Struct|BreakS_LevelData _currentleveldata))
  (bind (_value _returnvalue) (Utilities|Map|Find _cardamounts _name))
  (if _returnvalue
    (Utilities|Map|Add _cardamounts _name (- _value 1))))