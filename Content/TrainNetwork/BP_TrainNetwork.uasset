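; Rail actor for a train network that builds track meshes along its spline in the construction script, with no runtime logic.
; It divides the spline into sections sized from the actor's X scale and adds a spline mesh for each.
; Helper functions supply local start and end positions, with tangents clamped to section length so segments bend correctly.
; Each segment gets a dynamic M_Rail material instance tinted by the Color variable.
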(event EventBeginPlay)

(fn ConstructionScript
  (Variables|Default|SetSectionLength (* (.X (Math|Vector|BreakVector (Transformation|GetActorScale3D))) 1e+02))
  (for _index (range 0 (Math|Float|Truncate (/ (Spline|GetSplineLength (Variables|Default|GetSpline)) (Variables|Default|GetSectionLength))))
    (LocalVariables|SetLoopIndex _index)
    (bind _returnvalue (AddComponent|AddSplineMeshComponent false))
    (Components|StaticMesh|SetStaticMesh _returnvalue (Variables|Default|GetSplineMesh))
    (SplineMesh|SetForwardAxis _returnvalue "X" true)
    (bind (_pos _tan) (CallFunction|GetStartPosTangent (LocalVariables|GetLoopIndex)))
    (bind (_pos_2 _tan_2) (CallFunction|GetEndPosTangent (LocalVariables|GetLoopIndex)))
    (SplineMesh|SetStartandEnd _returnvalue _pos _tan _pos_2 _tan_2 true :!class /Script/Engine.SplineMeshComponent)
    (bind _returnvalue_2 (Rendering|Material|CreateDynamicMaterialInstance "/Game/TrainNetwork/M_Rail.M_Rail" "None" "None" :!class /Script/Engine.KismetMaterialLibrary))
    (Rendering|Material|SetMaterial _returnvalue 0 _returnvalue_2)
    (Rendering|Material|SetVectorParameterValue _returnvalue_2 "BaseColor" (Variables|Default|GetColor) :!class /Script/Engine.MaterialInstanceDynamic)))

(fn GetStartPosTangent
  (params (Index :type Integer))
  (bind _spline (Variables|Default|GetSpline))
  (bind _sectionlength (Variables|Default|GetSectionLength))
  (bind _returnvalue (* Index _sectionlength))
  (return (Spline|GetLocationatDistanceAlongSpline _spline _returnvalue "Local") (Math|Vector|ClampVectorSize (Spline|GetTangentatDistanceAlongSpline _spline _returnvalue "Local") 0.0 (Variables|Default|GetSectionLength))))

(fn GetEndPosTangent
  (params (Index :type Integer))
  (bind _returnvalue (+ Index 1))
  (bind _spline (Variables|Default|GetSpline))
  (bind _sectionlength (Variables|Default|GetSectionLength))
  (bind _returnvalue_2 (* _returnvalue _sectionlength))
  (return (Spline|GetLocationatDistanceAlongSpline _spline _returnvalue_2 "Local") (Math|Vector|ClampVectorSize (Spline|GetTangentatDistanceAlongSpline _spline _returnvalue_2 "Local") 0.0 (Variables|Default|GetSectionLength))))