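; Game mode for a train game that starts all trains and tracks the run's elapsed time, cards placed and trains finished.
; On begin play it binds to the director controller's card-placed event to keep the card count.
; StartTrains starts every BP_TrainNetwork and binds to its finish event, stopping the timer once all have finished.
; Reset reloads the current level.
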(event EventTick
  (params (DeltaSeconds :type Float%20%28single-precision%29))
  (if (Variables|Default|GetStarted)
    (Variables|Trackers|SetTimeSinceStart (+ (Variables|Trackers|GetTimeSinceStart) DeltaSeconds))))

(event EventBeginPlay
  (bind _asbp_train_director_controller (Utilities|Casting|CastToBP_TrainDirectorController (Game|GetPlayerController 0)))
  (EventDispatchers|BindEventtoCardPlaced _asbp_train_director_controller (EventDispatchers|CreateEvent :!event OnCardPlaced)))

(fn ConstructionScript)

(fn StartTrains
  (Variables|Default|SetStarted true)
  (bind _outactors (Actor|GetAllActorsOfClass "/Game/TrainNetwork/BP_TrainNetwork.BP_TrainNetwork_C"))
  (for _array_element _outactors
    (Default|StartTrain _array_element)
    (EventDispatchers|BindEventtoTrainFinished _array_element (EventDispatchers|CreateEvent :!event OnTrainFinished)))
  (Variables|Default|SetTrainCount (Utilities|Array|Length _outactors)))

(fn Reset
  (bind _returnvalue (Game|GetCurrentLevelName true))
  (Game|OpenLevel(byName) (Utilities|String|StringToName _returnvalue)))

(fn OnTrainFinished
  (bind _result (Math|Integer|IncrementInt (Variables|Trackers|GetCurrentTrainsFinished))
    (:%20%20
      (if (== _result (Variables|Default|GetTrainCount))
        (Variables|Default|SetStarted false)))))

(fn OnCardPlaced
  (Math|Integer|IncrementInt (Variables|Trackers|GetCurrentCardsPlaced)))