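; BP_BaseCardEffect is a base actor for card effects, showing a colored visual effect over a configurable radius.
; On BeginPlay it sizes its Sphere component to Radius without updating overlaps, then spawns the effect and moves itself to the Z of EffectHeight, keeping X and Y.
; SpawnCardEffect attaches the FXS_CardEffect system to the Sphere and passes Color and Radius in as effect parameters.
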(event EventBeginPlay
  (bind _returnvalue (Transformation|GetActorLocation))
  (bind (_x _y) (Math|Vector|BreakVector _returnvalue))
  (Components|Sphere|SetSphereRadius (Variables|Default|GetSphere) (Variables|Default|GetRadius) false)
  (CallFunction|SpawnCardEffect)
  (Transformation|SetActorLocation (Math|Vector|MakeVector _x _y (Variables|Default|GetEffectHeight)) false false))

(fn ConstructionScript)

(fn SpawnCardEffect
  (bind _returnvalue (Niagara|SpawnSystemAttached "/Game/Player/Cards/FXS_CardEffect.FXS_CardEffect" (Variables|Default|GetSphere) "None" "0, 0, 0" "0, 0, 0" "SnapToTarget" false))
  (Niagara|SetNiagaraVariable(LinearColor) _returnvalue "Color" (Variables|Default|GetColor))
  (Niagara|SetNiagaraVariable(Float) _returnvalue "Radius" (Variables|Default|GetRadius)))